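; Enemy spawner actor that spawns BP_Enemy instances at its own location and rotation, each given the DA_KA47 weapon.
; EnemySpawner spawns a given count in one loop, adjusting placement for collisions but always spawning.
; EnemyBatchSpawner calls it repeatedly, using a Delay loop to space batches by an interval.
; BeginPlay is empty and the sample batch call is disconnected, so nothing here triggers spawning.
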(event Custom|EnemySpawner
  (params (EnemyCount :type Integer))
  (Variables|Default|SetEnemyCount EnemyCount)
  (while (> (Variables|Default|GetEnemyCount) 0)
    (Game|SpawnActorfromClass "/Game/Blueprints/BP_Enemy.BP_Enemy_C" (Math|Transform|MakeTransform (Transformation|GetActorLocation) (Transformation|GetActorRotation) "1.000000,1.000000,1.000000") "AdjustIfPossibleButAlwaysSpawn" "MultiplyWithRoot" 0 "/Game/Weapon/DataAssetSkeletal/DA_KA47.DA_KA47" 0)
    (Variables|Default|SetEnemyCount (- (Variables|Default|GetEnemyCount) 1))))

(event Custom|EnemyBatchSpawner
  (params (TotalBatch :type Integer) (EnemyCount :type Integer) (Interval :type Float%20%28double-precision%29))
  (Variables|Default|SetBatch TotalBatch)
  (CallFunction|EnemySpawner EnemyCount :!label _label)
  (Variables|Default|SetBatch (- (Variables|Default|GetBatch) 1))
  (if (> (Variables|Default|GetBatch) 0)
    (Utilities|FlowControl|Delay Interval)
    (goto _label)))

(event EventBeginPlay)

(fn ConstructionScript)