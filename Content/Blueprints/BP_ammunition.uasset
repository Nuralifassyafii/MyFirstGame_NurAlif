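; BP_ammunition is a pickup actor that gives extra magazines to a player character on overlap.
; It casts the overlapping actor to BP_ThirdPersonCharacterBase and checks whether its current magazines plus AddMagz stay within the weapon's MaxMagz.
; If they fit, it adds them and destroys itself; otherwise it stays and prints an "ammo still full" message in Indonesian.
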(event EventBeginPlay)

(event Collision|EventActorBeginOverlap
  (params (OtherActor :type Actor%20Object%20Reference))
  (bind _asbp_third_person_character_base (Utilities|Casting|CastToBP_ThirdPersonCharacterBase OtherActor))
  (if (<= (+ (Variables|/Game/Characters/Character_mixamo/BP_ThirdPersonCharacterBase.BP_ThirdPersonCharacterBase_C|GetMagz _asbp_third_person_character_base) (Variables|Default|GetaddMagz)) (Variables|/Game/Weapon/DataAssetSkeletal/BP_weapon_data_skeletal.BP_weapon_data_skeletal_C|GetMaxMagz (Variables|/Game/Characters/Character_mixamo/BP_ThirdPersonCharacterBase.BP_ThirdPersonCharacterBase_C|GetWeaponSkeletal _asbp_third_person_character_base)))
    (Default|AddMagz _asbp_third_person_character_base (Variables|Default|GetaddMagz))
    (Actor|DestroyActor)
    (else
      (Development|PrintString "ammo masih penuh"))))

(fn ConstructionScript)