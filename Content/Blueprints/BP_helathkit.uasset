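; BP_helathkit is a health pickup actor that heals a third-person character who overlaps it.
; On overlap it casts to BP_ThirdPersonCharacterBase, calls AddHealth with HealthMedkit, then destroys itself.
; It heals only when the full amount fits within MaxHealth; otherwise it stays and prints an Indonesian "health still full" message, even if the character is slightly hurt.
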(event EventBeginPlay)

(event Collision|EventActorBeginOverlap
  (params (OtherActor :type Actor%20Object%20Reference))
  (bind _asbp_third_person_character_base (Utilities|Casting|CastToBP_ThirdPersonCharacterBase OtherActor))
  (if (<= (+ (Variables|/Game/Characters/Character_mixamo/BP_ThirdPersonCharacterBase.BP_ThirdPersonCharacterBase_C|Gethealth _asbp_third_person_character_base) (Variables|Default|GetHealthMedkit)) (Variables|/Game/Characters/Character_mixamo/BP_ThirdPersonCharacterBase.BP_ThirdPersonCharacterBase_C|GetmaxHealth _asbp_third_person_character_base))
    (Default|AddHealth _asbp_third_person_character_base (Variables|Default|GetHealthMedkit))
    (Actor|DestroyActor)
    (else
      (Development|PrintString "health masih penuh"))))

(fn ConstructionScript)